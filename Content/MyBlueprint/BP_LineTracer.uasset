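; BP_LineTracer is a one-shot probe actor that places a BP_DissolveCube where nothing occupies the ground below it.
; On BeginPlay it traces downward along its up vector on the Visibility channel.
; If the trace misses, it increments the object count on BP_TracerSpawner and spawns the cube at its X/Y with a fixed height.
; It destroys itself afterward either way.
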(event Custom|CheckObj
  (bind _defaultsceneroot (Variables|Default|GetDefaultSceneRoot))
  (bind _returnvalue (Transformation|GetWorldLocation _defaultsceneroot))
  ;[1 1 1] Send rays downward to detect if there is an occlusion
  (bind _returnvalue_2 (Collision|LineTraceByChannel _returnvalue (+ _returnvalue (* (* (Math|Vector|GetUpVector (Variables|Default|GetDefaultSceneRoot)) (Variables|Default|GetLineDis)) -1.0)) "TraceTypeQuery1" false 0 "None"))
  (Variables|Default|SethaveObj _returnvalue_2))

(event EventBeginPlay
  (bind _defaultsceneroot (Variables|Default|GetDefaultSceneRoot))
  (bind _returnvalue (Transformation|GetWorldTransform _defaultsceneroot))
  (CallFunction|CheckObj)
  (if (Variables|Default|GethaveObj)
    _
    (else
      ;[1 1 1] Create a cube and add 1 to the count
      (bind _returnvalue_2 (Actor|GetActorOfClass "/Game/MyBlueprint/BP_TracerSpawner.BP_TracerSpawner_C"))
      (Variables|/Game/MyBlueprint/BP_TracerSpawner.BP_TracerSpawner_C|SetobjNumInLevel _returnvalue_2 (+ (Variables|/Game/MyBlueprint/BP_TracerSpawner.BP_TracerSpawner_C|GetobjNumInLevel _returnvalue_2) 1))
      (Game|SpawnActorfromClass "/Game/MyBlueprint/BP_DissolveCube.BP_DissolveCube_C" (Math|Conversions|ToTransform(Vector) (Math|Vector|MakeVector (.x (.location _returnvalue)) (.y (.location _returnvalue)) 5e+01)) "Undefined" 0 0)))
  (Actor|DestroyActor))

(event Collision|EventActorBeginOverlap
  (params (OtherActor :type Actor%20Object%20Reference)))

(event EventTick
  (params (DeltaSeconds :type Float%20%28single-precision%29)))

(fn ConstructionScript)