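; BP_DissolveCube is a cube actor that wanders in grid steps and dissolves when a Player-tagged component hits it.
; Periodic line traces in four directions collect open slots, and Tick moves the cube toward a random one.
; Hits from components tagged neither Player nor Ground stop movement.
; A timeline drives the material and Niagara dissolve, then decrements BP_TracerSpawner's object count, triggers its count check and destroys the cube.
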(event OnComponentHit(Cube)
  (params (HitComponent :type Primitive%20Component%20Object%20Reference) (OtherActor :type Actor%20Object%20Reference) (OtherComp :type Primitive%20Component%20Object%20Reference) (NormalImpulse :type Vector :default "0, 0, 0") (Hit :type Hit%20Result%20Structure%20%28by%20ref%29))
  ;[1 1 1] If the player hits the cube, start dissolving
  ;[0.5874 1 0.4992] Change to use tag to detect object collisions.
  (if (Components|ComponentHasTag OtherComp "Player")
    (if (not (Variables|Default|GetisDissolved))
      (Variables|Default|SetisDissolved true)
      (CallFunction|Dissolving))
    (elif (not (Components|ComponentHasTag OtherComp "Ground"))
      (Variables|Default|SetcanMove false))))

(event Custom|Dissolving
  ;[1 1 1] Using timeline to control the dissolve animation
  (bind _tl_leaking (Timeline|Timeline_0 Play)
    (:Update
      (Rendering|Material|SetScalarParameterValueonMaterials (Variables|Default|GetCube) "dissolve" _tl_leaking)
      (Niagara|SetNiagaraVariable(Float) (Variables|Default|GetNiagara) "User_dissolve" _tl_leaking))
    (:Finished
      ;[1 1 1] Decrease the count by 1 when the cube disappears
      (bind _returnvalue (Actor|GetActorOfClass "/Game/MyBlueprint/BP_TracerSpawner.BP_TracerSpawner_C"))
      (Variables|/Game/MyBlueprint/BP_TracerSpawner.BP_TracerSpawner_C|SetobjNumInLevel _returnvalue (- (Variables|/Game/MyBlueprint/BP_TracerSpawner.BP_TracerSpawner_C|GetobjNumInLevel _returnvalue) 1))
      (Default|CheckObjNum _returnvalue)
      (Actor|DestroyActor))))

(event Custom|CheckAround
  ;[0.5874 1 0.4992] Empty the set and detect it once in all four directions.
  (Utilities|Array|Clear (Variables|Default|GetSlotsAround))
  (CallFunction|LineTrace (Class|KismetMathLibrary|VectorForward))
  (CallFunction|LineTrace (Class|KismetMathLibrary|VectorBackward))
  (CallFunction|LineTrace (Class|KismetMathLibrary|VectorLeft))
  (CallFunction|LineTrace (Class|KismetMathLibrary|VectorRight))
  ;[0.5874 1 0.4992] Random selection of a moveable direction
  (Variables|Default|SetmoveVector (.OutItem (Utilities|Array|Random (Variables|Default|GetSlotsAround))))
  ;[0.5874 1 0.4992] Sets the move target and determines if it can be moved by determining if the moveable set is empty.
  (Variables|Default|SettargetPos (+ (Transformation|GetWorldLocation (Variables|Default|GetCube)) (* (Variables|Default|GetmoveVector) 2e+02)))
  (if (Utilities|Array|IsNotEmpty (Variables|Default|GetSlotsAround))
    (Variables|Default|SetcanMove true)))

(event Custom|TryMove
  ;[0.5874 1 0.4992] Move when it is possible to do so
  (if (Variables|Default|GetcanMove)
    (Transformation|AddWorldOffset (Variables|Default|GetCube) (* (* (Variables|Default|GetmoveVector) (Variables|Default|GetmoveSpeed)) (Utilities|Time|GetWorldDeltaSeconds)) false false)
    ;[0.5874 1 0.4992] Change to immovable on arrival at target
    (if (<= (Math|Vector|VectorLength (- (Transformation|GetWorldLocation (Variables|Default|GetCube)) (Variables|Default|GettargetPos))) 0.5)
      (Variables|Default|SetcanMove false))))

(event EventTick
  (params (DeltaSeconds :type Float%20%28single-precision%29))
  ;[0.5874 1 0.4992] Check around every once in a while to make sure it's ready to move
  (CallFunction|TryMove)
  (Utilities|FlowControl|Delay (Variables|Default|GetDuration))
  (CallFunction|CheckAround))

(fn ConstructionScript)

(fn LineTrace
  (params (Vector :type Vector))
  (bind _cube (Variables|Default|GetCube))
  (bind _returnvalue (Transformation|GetWorldLocation _cube))
  (bind _returnvalue_2 (Collision|LineTraceByChannel _returnvalue (+ _returnvalue (* Vector 2e+02)) "TraceTypeQuery1" false 0 "None"))
  (if (not _returnvalue_2)
    (Utilities|Array|Add (Variables|Default|GetSlotsAround) Vector)))