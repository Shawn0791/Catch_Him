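; BP_DissolveChar is a catch-me target character that roams to random points while evading BP_ThirdPersonCharacter.
; Tick drives vector-based steering with dot and cross products, choosing to head to the target, circle around the player or flee, and re-rolling targets when reached or near the player.
; A player hit enables ragdoll physics and a timeline-driven material and Niagara dissolve, then spawns a replacement at a random spot and destroys itself.
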(event OnComponentHit(SkeletalMesh)
  (params (HitComponent :type Primitive%20Component%20Object%20Reference) (OtherActor :type Actor%20Object%20Reference) (OtherComp :type Primitive%20Component%20Object%20Reference) (NormalImpulse :type Vector :default "0, 0, 0") (Hit :type Hit%20Result%20Structure%20%28by%20ref%29))
  ;[1 1 1] If the player hits the character, start dissolving
  (Utilities|Casting|CastToBP_ThirdPersonCharacter OtherActor)
  (if (not (Variables|Default|GetisDissolved))
    (Variables|Default|SetisDissolved true)
    (CallFunction|Dissolving)
    (CallFunction|GetHit)))

(event Custom|Dissolving
  ;[1 1 1] Using timeline to control the dissolve animation
  (bind _tl_leaking (Timeline|Timeline Play)
    (:Update
      (Rendering|Material|SetScalarParameterValueonMaterials (Variables|Default|GetSkeletalMesh) "dissolve" _tl_leaking)
      (Niagara|SetNiagaraVariable(Float) (Variables|Default|GetNiagara) "User_dissolve" _tl_leaking))
    (:Finished
      ;[1 1 1] Spawns a character at a random position after the timeline ends
      (Game|SpawnActorfromClass "BP_DissolveChar_C" (Math|Conversions|ToTransform(Vector) (Math|Vector|MakeVector (* (Math|Random|RandomIntegerinRange -9 9) 2e+02) (* (Math|Random|RandomIntegerinRange -9 9) 2e+02) 5e+01)) "Undefined" 0 0)
      (Development|PrintString "He's coming again, catch him !!!" true true "(R=1.000000,G=0.000000,B=0.035645,A=1.000000)")
      (Actor|DestroyActor))))

(event Custom|GetHit
  ;[1 1 1] Received an attack to stop animation and start physics simulation
  (Components|Animation|SetAnimation (Variables|Default|GetSkeletalMesh) 0)
  (Physics|SetSimulatePhysics (Variables|Default|GetSkeletalMesh) true)
  (Development|PrintString "Well done ~" true true "(R=0.000000,G=1.000000,B=0.093912,A=1.000000)"))

(event Custom|CharMovement_New
  (bind _returnvalue (Transformation|GetActorLocation))
  (bind _returnvalue_2 (Math|Vector|VectorUp))
  (bind _returnvalue_3 (Transformation|GetActorLocation))
  (bind _playerpos (Variables|Default|GetplayerPos))
  (bind _targetpos (Variables|Default|GettargetPos))
  (bind _returnvalue_4 (- _targetpos _returnvalue_3))
  (bind _returnvalue_5 (- _playerpos _returnvalue))
  (bind _returnvalue_6 (Math|Vector|Normalize _returnvalue_4))
  (bind _returnvalue_7 (Math|Vector|CrossProduct _returnvalue_5 _returnvalue_2))
  ;[0.5874 1 0.4992] PT<=R, ChangePos
  (if (<= (Math|Vector|VectorLength (- (Variables|Default|GetplayerPos) (Variables|Default|GettargetPos))) (Variables|Default|GetRange))
    (Utilities|RandomTarget)
    (else
      ;[0.5874 1 0.4992] PT>R & Clamping angle<=90
      (if (<= (Math|Vector|DotProduct (- (Variables|Default|GetplayerPos) (Transformation|GetActorLocation)) (- (Variables|Default|GettargetPos) (Transformation|GetActorLocation))) 0.0)
        (Utilities|MoveToward (Utilities|TargetDistance))
        (else
          ;[0.5874 1 0.4992] PT>R & Clamping angle>90 & PM>=R
          (if (>= (/ (Math|Vector|VectorLength (Math|Vector|CrossProduct (- (Variables|Default|GetplayerPos) (Transformation|GetActorLocation)) _returnvalue_6)) (Math|Vector|VectorLength _returnvalue_6)) (Variables|Default|GetRange))
            (Utilities|MoveToward (Utilities|TargetDistance))
            (else
              ;[0.5874 1 0.4992] Determining whether to run away
              (if (Variables|Default|GetrunAway)
                (Utilities|MoveToward (- (Transformation|GetActorLocation) (Variables|Default|GetplayerPos)))
                (if (> (Math|Vector|VectorLength (- (Variables|Default|GetplayerPos) (Transformation|GetActorLocation))) (+ (Variables|Default|GetRange) 5e+02))
                  (Variables|Default|SetrunAway false))
                (else
                  ;[0.5874 1 0.4992] PT>R & Clamping angle>90 & PM<R & EP>R
                  (if (> (Math|Vector|VectorLength (- (Variables|Default|GetplayerPos) (Transformation|GetActorLocation))) (+ (Variables|Default|GetRange) (Variables|Default|GetrangeOffset)))
                    (Utilities|MoveToward (Utilities|TargetDistance))
                    (else
                      ;[0.5874 1 0.4992] PT>R & Clamping angle>90 & PM<R & EP<R
                      (if (< (Math|Vector|VectorLength (- (Variables|Default|GetplayerPos) (Transformation|GetActorLocation))) (- (Variables|Default|GetRange) (Variables|Default|GetrangeOffset)))
                        (Variables|Default|SetrunAway true)
                        (else
                          ;[0.5874 1 0.4992] PT>R & Clamping angle>90 & PM<R & EP=R
                          (if (> (Math|Vector|DotProduct _returnvalue_7 (- (Variables|Default|GettargetPos) (Transformation|GetActorLocation))) 0.0)
                            (Utilities|MoveToward _returnvalue_7)
                            (else
                              (Utilities|MoveToward (* _returnvalue_7 -1.0)))))))))))))))))

(event Custom|CharMovement
  ;[1 1 1] Character movement
  (Transformation|AddActorWorldOffset (* (* (Variables|Default|GetmoveSpeed) (Utilities|Time|GetWorldDeltaSeconds)) (Math|Vector|Normalize (Utilities|TargetDistance))))
  ;[1 1 1] Face to target
  (Transformation|SetActorRotation (Math|Rotator|MakeRotfromX (Utilities|TargetDistance))))

(event Custom|CheckDis
  ;[1 1 1] Check the distance between the character and the target, and randomly change the target position if it is close enough
  (if (<= (Math|Vector|VectorLength (Utilities|TargetDistance)) 15.0)
    (Utilities|RandomTarget)))

(event EventBeginPlay
  (Utilities|RandomTarget)
  (bind _returnvalue (Actor|GetActorOfClass "/Game/ThirdPerson/Blueprints/BP_ThirdPersonCharacter.BP_ThirdPersonCharacter_C")))

(event EventTick
  (params (DeltaSeconds :type Float%20%28single-precision%29))
  ;[0.5874 1 0.4992] Determine the player's position and execute the move function
  (CallFunction|CheckDis)
  (CallFunction|CharMovementNew)
  (Variables|Default|SetplayerPos (Transformation|GetActorLocation (stale EventBeginPlay _returnvalue))))

(fn ConstructionScript)