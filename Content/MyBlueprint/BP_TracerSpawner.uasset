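; BP_TracerSpawner fills the level with BP_LineTracer actors at timed intervals and runs game start (message) and Escape-to-quit.
; BeginPlay builds a grid of positions, then StartSpawn loops until MaxObjNum; CheckObjNum restarts it below MinObjNum.
; Each spawn draws from that pool and removes an entry, but separate Random calls may remove a different position.
; ObjNumInLevel is only reset here, and the older random-coordinate SpawnOnce is unused.
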(event Custom|SpawnOnce
  (Game|SpawnActorfromClass "/Game/MyBlueprint/BP_LineTracer.BP_LineTracer_C" (Math|Conversions|ToTransform(Vector) (Math|Vector|MakeVector (* (Math|Random|RandomIntegerinRange -9 9) 2e+02) (* (Math|Random|RandomIntegerinRange -9 9) 2e+02) 5e+02)) "Undefined" 0 0))

(event Custom|StartSpawn
  ;[1 1 1] Always create cubes until the number of cubes reaches the maximum value
  (if (< (Variables|Default|GetobjNumInLevel) (Variables|Default|GetMaxObjNum)) :!label _label
    (CallFunction|SpawnOnceNew)
    (Utilities|FlowControl|Delay (/ 1.0 (Variables|Default|GetSpawnSpeed)))
    (goto _label)))

(event Custom|CheckObjNum
  ;[1 1 1] If the number of cubes is less than the minimum value, increase to the maximum value
  (if (< (Variables|Default|GetobjNumInLevel) (Variables|Default|GetMinObjNum))
    (CallFunction|StartSpawn)))

(event Custom|AddPos
  ;[0.5874 1 0.4992] Add each of the locations that can be generated to the set according to the size of the map.
  (for _index (range -9 9)
    (for _index_2 (range -9 9)
      (Utilities|Array|Add (Variables|Default|GetPositions) (Math|Conversions|ToTransform(Vector) (Math|Vector|MakeVector (* _index_2 200) (* _index 200) 5e+02))))))

(event Custom|SpawnOnce_New
  (bind _positions (Variables|Default|GetPositions))
  (bind (_outitem _outindex) (Utilities|Array|Random _positions))
  ;[0.5874 1 0.4992] A randomly selected position within the set is generated and the position is removed from the set when generation is complete.
  (Game|SpawnActorfromClass "/Game/MyBlueprint/BP_LineTracer.BP_LineTracer_C" _outitem "Undefined" 0 0)
  (Utilities|Array|RemoveIndex (Variables|Default|GetPositions) _outindex))

(event EventBeginPlay
  ;[0.5874 1 0.4992] At the start of the game, add all the dots and then start generating obstacles.
  (Variables|Default|SetobjNumInLevel 0)
  (CallFunction|AddPos)
  (CallFunction|StartSpawn)
  (Development|PrintString "Catch the white guy !!!" true true "(R=1.000000,G=0.000000,B=0.050402,A=1.000000)"))

(event Collision|EventActorBeginOverlap
  (params (OtherActor :type Actor%20Object%20Reference)))

(event EventTick
  (params (DeltaSeconds :type Float%20%28single-precision%29)))

(event Input|KeyboardEvents|Escape
  (params (Key :type Key%20Structure :default "None"))
  (:Pressed
    (Game|QuitGame 0 "Quit" false)))

(fn ConstructionScript)