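; Wind audio Blueprint that varies its AudioComponent's sound over time to create gusts.
; Every Tick, slowly sampled 1D Perlin noise of game time drives both volume and low-pass filter frequency, so louder moments also sound brighter.
; Math expressions shape the noise, using a cubic curve for volume and an exponential, octave-style mapping for the filter cutoff.
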(event EventBeginPlay)

(event EventTick
  (params (DeltaSeconds :type Float%20%28single-precision%29))
  (bind _returnvalue (Utilities|Time|GetTimeSeconds))
  (bind _returnvalue_2 (* _returnvalue 0.2))
  (bind _returnvalue_3 (Class|KismetMathLibrary|PerlinNoise1D _returnvalue_2))
  (Audio|Components|Audio|SetVolumeMultiplier (Variables|Components|GetAudioComponent) (|(pow(((x*0.500000)+0.500000),3)) _returnvalue_3) :!class /Script/Engine.AudioComponent)
  (Audio|Components|Audio|SetLowPassFilterFrequency (Variables|Components|GetAudioComponent) (|((pow(2,(2*x)))*1000) _returnvalue_3) :!class /Script/Engine.AudioComponent))

(fn ConstructionScript)